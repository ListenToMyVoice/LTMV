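; Lobby trigger actor that starts the match when a PlayerCharacterRed overlaps it.
; The overlap runs only on the server, where it casts the game mode to GameModeLobby and calls LaunchGame.
; On BeginPlay it sets the first player controller to Game and UI input, focusing the widget hosted by its StartMenu component.
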(event EventBeginPlay
  (Input|SetInputModeGameandUI (Game|GetPlayerController 0) (UserInterface|GetUserWidgetObject (Variables|Default|GetStartMenu)) "DoNotLock" false))

(event EventTick
  (params (DeltaSeconds :type Float%20%28single-precision%29)))

(event Collision|EventActorBeginOverlap
  (params (OtherActor :type Actor%20Object%20Reference))
  ;[1 1 1] Start Match
  (Utilities|Casting|CastToPlayerCharacterRed OtherActor)
  (if (Networking|IsServer)
    (bind _asgame_mode_lobby (Utilities|Casting|CastToGameModeLobby (Game|GetGameMode)))
    (Class|GameModeLobby|LaunchGame _asgame_mode_lobby)))

(fn ConstructionScript)