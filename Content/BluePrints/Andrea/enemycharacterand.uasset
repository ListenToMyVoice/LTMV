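; Enemy character Blueprint that patrols between two points and detects the player, feeding both to its AI Blackboard.
; On begin play it writes CurrentPatrolPoint to the PatrolPoint key.
; Overlapping either patrol point switches the current target to the other and updates that key.
; PawnSensing stores a seen PlayerCharacter in the PlayerActor key, which is never cleared here.
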(event OnSeePawn(PawnSensing)
  (params (Pawn :type Pawn%20Object%20Reference))
  ;[1 1 1] When player is seen, store that knowledge in the Blackboard
  (bind _asplayer_character (Utilities|Casting|CastToPlayerCharacter Pawn))
  (AI|Components|Blackboard|SetValueasObject (AI|GetBlackboard self) (Utilities|Name|MakeLiteralName "PlayerActor") _asplayer_character))

(event EventBeginPlay
  ;[1 1 1] When enemy is created, set blackboard key to Patrol Point
  (AI|Components|Blackboard|SetValueasObject (AI|GetBlackboard self) (Utilities|Name|MakeLiteralName "PatrolPoint") (Variables|Default|GetCurrentPatrolPoint)))

(event Collision|EventActorBeginOverlap
  (params (OtherActor :type Actor%20Object%20Reference))
  ;[1 1 1] Set CurrentPatrolPoint to the patrol point not currently being overlapped
  (if (== OtherActor (Variables|Default|GetPatrolPoint1))
    (Variables|Default|SetCurrentPatrolPoint (Variables|Default|GetPatrolPoint2))
    ;[1 1 1] When enemy is created, set blackboard key to Patrol Point
    (AI|Components|Blackboard|SetValueasObject (AI|GetBlackboard self) (Utilities|Name|MakeLiteralName "PatrolPoint") (Variables|Default|GetCurrentPatrolPoint) :!label _label)
    (elif (== OtherActor (Variables|Default|GetPatrolPoint2))
      (Variables|Default|SetCurrentPatrolPoint (Variables|Default|GetPatrolPoint1))
      (goto _label))))

(event EventTick
  (params (DeltaSeconds :type Float%20%28single-precision%29)))

(fn ConstructionScript)