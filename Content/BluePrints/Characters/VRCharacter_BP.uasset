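; VR character Blueprint that keeps the animated hand meshes in step with each hand's grip state.
; Every Tick, it casts the left and right hand meshes' anim instances to RightHand_AnimBP and copies GripStateLeft and GripStateRight into their GripState.
; Both hands share the RightHand_AnimBP class, and the grip states are only read here, with no input logic or construction logic.
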(event EventTick
  (params (DeltaSeconds :type Float%20%28single-precision%29))
  (Utilities|FlowControl|Sequence
    (:then_0
      (bind _asright_hand_anim_bp (Utilities|Casting|CastToRightHand_AnimBP (Components|SkeletalMesh|GetAnimInstance (Variables|Default|Get_SM_LeftHand))))
      (Variables|/Game/Meshes/Skeletons/VRPlayer/Animations/RightHand_AnimBP.RightHand_AnimBP_C|SetGripState _asright_hand_anim_bp (Variables|Default|Get_GripStateLeft)))
    (:then_1
      (bind _asright_hand_anim_bp_2 (Utilities|Casting|CastToRightHand_AnimBP (Components|SkeletalMesh|GetAnimInstance (Variables|Default|Get_SM_RightHand))))
      (Variables|/Game/Meshes/Skeletons/VRPlayer/Animations/RightHand_AnimBP.RightHand_AnimBP_C|SetGripState _asright_hand_anim_bp_2 (Variables|Default|Get_GripStateRight)))))

(fn ConstructionScript)