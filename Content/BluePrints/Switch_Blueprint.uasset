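; Switch Blueprint that toggles a set of point lights on and off when its Use event fires.
; Its Toggle object holds parallel arrays of actors and states.
; Use first inverts and stores every state, then applies each one as light component visibility to the actor at the same index.
; Only actors that cast to PointLight are affected, and visibility does not propagate to children.
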(event EventUse
  (bind _toggle (Variables|Default|GetToggle))
  (bind _returnvalue (Class|Toggle|GetArrayOfStates (Variables|Default|GetToggle)))
  (for (_array_element _array_index) _returnvalue
    (bind _returnvalue_2 (Class|Toggle|InvertState (Variables|Default|GetToggle) _array_element))
    (Class|Toggle|SetState (Variables|Default|GetToggle) _returnvalue_2 _array_index))
  (bind _returnvalue_3 (Class|Toggle|GetArrayOfActors _toggle))
  (bind _returnvalue_4 (Class|Toggle|GetArrayOfStates _toggle))
  (for (_array_element_2 _array_index_2) _returnvalue_3
    (bind _aspoint_light (Utilities|Casting|CastToPointLight _array_element_2))
    (Rendering|SetVisibility (Variables|/Script/Engine.Light|GetLightComponent _aspoint_light) (Utilities|Array|Get(acopy) _returnvalue_4 _array_index_2) false)))

(fn ConstructionScript)