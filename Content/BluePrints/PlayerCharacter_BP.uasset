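; PlayerCharacter_BP is the player character Blueprint that handles using objects in the world and clicking on widgets.
; The Use input calls the ServerAttemptUseFunction event, which runs a raycast and sends UseMessage to a blocking hit actor that implements the ItfUsable interface.
; Left mouse press and release are forwarded to a WidgetInteraction component as pointer key events.
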(event Custom|ServerAttemptUseFunction
  (CallFunction|AttemptUseFunction))

(event Input|ActionEvents|InputActionUse
  (params (Key :type Key%20Structure :default "AnyKey"))
  (:Pressed
    (CallFunction|ServerAttemptUseFunction)))

(event Input|MouseEvents|LeftMouseButton
  (params (Key :type Key%20Structure :default "AnyKey"))
  (bind _widgetinteraction (Variables|Default|GetWidgetInteraction))
  (:Pressed
    (Class|WidgetInteractionComponent|PressPointerKey _widgetinteraction "LeftMouseButton"))
  (:Released
    (Class|WidgetInteractionComponent|ReleasePointerKey _widgetinteraction "LeftMouseButton")))

(fn ConstructionScript)

(fn AttemptUseFunction
  (bind _returnvalue (Class|PlayerCharacter|Raycasting))
  (if (and (.bBlockingHit (Collision|BreakHitResult _returnvalue)) (Utilities|DoesObjectImplementInterface (.HitActor (Collision|BreakHitResult _returnvalue)) "/Script/proyecto.ItfUsable"))
    (Class|ItfUsable|Use(Message) (.HitActor (Collision|BreakHitResult _returnvalue)))))