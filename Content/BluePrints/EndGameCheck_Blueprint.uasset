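; EndGameCheck is an overlap-driven actor that starts the end-game effect once two player characters are inside it at the same time.
; Begin and end overlap events filter for PlayerCharacter and raise or lower a shared counter.
; When an entry brings the count to exactly two, it spawns EndGameFX_Blueprint at a hard-coded world transform, with no guard against spawning again on re-entry.
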(event Collision|EventActorBeginOverlap
  (params (OtherActor :type Actor%20Object%20Reference))
  (Utilities|Casting|CastToPlayerCharacter OtherActor)
  (bind _output_get (Variables|Default|SetCounter (+ (Variables|Default|GetCounter) 1)))
  (if (== _output_get 2)
    (Game|SpawnActorfromClass "/Game/BluePrints/EndGameFX_Blueprint.EndGameFX_Blueprint_C" (Math|Transform|MakeTransform "4000.000000,-550.000000,150.000000" "0,-180.000000, 0") "Undefined" 0 0)))

(event Collision|EventActorEndOverlap
  (params (OtherActor :type Actor%20Object%20Reference))
  (Utilities|Casting|CastToPlayerCharacter OtherActor)
  (Variables|Default|SetCounter (- (Variables|Default|GetCounter) 1)))

(fn ConstructionScript)