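; Sky Blueprint that drives a day-night cycle by rotating a Sun actor over time.
; BeginPlay converts DayLength from minutes into the real seconds that make up one in-game hour.
; Tick advances Time in hours, maps it to a sun pitch of 15 degrees per hour with a 90-degree offset, then calls UpdateSunDirection on the Sky reference.
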(event EventBeginPlay
  (bind _output_get (Variables|Default|SetDay (* (Variables|Default|GetDayLength) 6e+01)))
  (Variables|Default|SetHour (/ _output_get 24.0)))

(event EventTick
  (params (DeltaSeconds :type Float%20%28single-precision%29))
  (bind _output_get (Variables|Default|SetTime (+ (Variables|Default|GetTime) (/ DeltaSeconds (Variables|Default|GetHour)))))
  (bind _output_get_2 (Variables|Default|SetSunAngle (+ (* (/ _output_get 6.0) 9e+01) 9e+01)))
  (Transformation|SetActorRotation (Variables|Default|GetSun) (Math|Rotator|MakeRotator 0.0 _output_get_2 0.0))
  (Default|UpdateSunDirection (Variables|Default|GetSky)))

(fn ConstructionScript)