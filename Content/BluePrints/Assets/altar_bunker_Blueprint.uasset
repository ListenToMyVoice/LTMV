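; Bunker altar that unblocks the final wall once the world's tablet (Tablilla) is placed in its token holder.
; On BeginPlay it caches the first tablet actor and the DoorState of the first actor in its Switcher list.
; Box overlap flags possession if an FP character holds or stores the tablet, or a VR character has it attached.
; Once flagged, Tick polls the TokenHolder and clears the door's Block when the tablet matches.
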(event OnComponentBeginOverlap(Box)
  (params (OverlappedComponent :type Primitive%20Component%20Object%20Reference) (OtherActor :type Actor%20Object%20Reference) (OtherComp :type Primitive%20Component%20Object%20Reference) (OtherBodyIndex :type Integer) (bFromSweep :type Boolean) (SweepResult :type Hit%20Result%20Structure%20%28by%20ref%29))
  (bind _asfpcharacter (Utilities|Casting|CastToFPCharacter OtherActor)
    (:then
      (bind _returnvalue (Class|PlayerCharacter|GetItemLeft _asfpcharacter))
      (if (== _returnvalue (Variables|Default|GetTablillaMundo))
        (Variables|Default|SetHasTablilla true :!label _label)
        (else
          (bind _returnvalue_2 (Class|PlayerCharacter|GetItemRight _asfpcharacter))
          (if (== _returnvalue_2 (Variables|Default|GetTablillaMundo))
            (goto _label)
            (else
              (bind _returnvalue_3 (Class|Inventory|GetItemsArray (Variables|/Script/LTMV.FPCharacter|Get_Inventory _asfpcharacter)))
              (bind _array_element (Utilities|Array|ForEachLoopwithBreak _returnvalue_3)
                (:LoopBody
                  (if (== _array_element (Variables|Default|GetTablillaMundo))
                    (goto _label)))))))))
    (:CastFailed
      (bind _asvrcharacter (Utilities|Casting|CastToVRCharacter OtherActor))
      (bind _array_element_2 (Utilities|Array|ForEachLoopwithBreak (Actor|GetAttachedActors _asvrcharacter))
        (:LoopBody
          (if (== _array_element_2 (Variables|Default|GetTablillaMundo))
            (goto _label)))))))

(event EventBeginPlay
  (Variables|Default|SetHasTablilla false)
  (bind _outactors (Actor|GetAllActorsOfClass "/Game/BluePrints/Assets/tablilla_bunker_Blueprint.tablilla_bunker_Blueprint_C"))
  (bind _array_element (Utilities|Array|ForEachLoopwithBreak _outactors :!label _label)
    (:LoopBody
      (Variables|Default|SetTablillaMundo _array_element)
      (goto _label Break))
    (:Completed
      (bind _array_element_2 (Utilities|Array|ForEachLoopwithBreak (Utilities|Struct|BreakSwitcher (Variables|/Script/LTMV.SwitcherComponent|Get_Switcher (Variables|Default|GetSwitcher))) :!label _label_2)
        (:LoopBody
          (Variables|Default|SetDoorState_MuroFinal (Actor|GetComponentbyClass (._actor (Utilities|Struct|BreakSwitcheable _array_element_2)) "/Script/LTMV.DoorState"))
          (goto _label_2 Break))))))

(event EventTick
  (params (DeltaSeconds :type Float%20%28single-precision%29))
  (if (Variables|Default|GetHasTablilla)
    (if (== (Variables|/Script/LTMV.TokenHolder|Get_Tablilla (Variables|Default|GetTokenHolder)) (Variables|Default|GetTablillaMundo))
      (Variables|/Script/LTMV.DoorState|Set_block (Variables|Default|GetDoorState_MuroFinal) false))))

(fn ConstructionScript)