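; Labyrinth altar that takes the tagged tablet (Tablilla) and unblocks the final wall's door.
; BeginPlay caches the first tagged tablet and the DoorState of the first actor in UseSwitcher's switchable list.
; Box overlap latches HasTablilla by checking an FPCharacter's hands and inventory, or a VRCharacter's tagged mesh components.
; UsePressed, if the flag is set and the tablet is equipped, clears the door block and snaps the tablet to TablillaSocket.
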(event OnComponentBeginOverlap(Box)
  (params (OverlappedComponent :type Primitive%20Component%20Object%20Reference) (OtherActor :type Actor%20Object%20Reference) (OtherComp :type Primitive%20Component%20Object%20Reference) (OtherBodyIndex :type Integer) (bFromSweep :type Boolean) (SweepResult :type Hit%20Result%20Structure%20%28by%20ref%29))
  (bind _asfpcharacter (Utilities|Casting|CastToFPCharacter OtherActor)
    (:then
      (bind _returnvalue (Class|PlayerCharacter|GetItemLeft _asfpcharacter))
      (if (== _returnvalue (Variables|Default|GetTablilla))
        (Variables|Default|SetHasTablilla true :!label _label)
        (else
          (bind _returnvalue_2 (Class|PlayerCharacter|GetItemRight _asfpcharacter))
          (if (== _returnvalue_2 (Variables|Default|GetTablilla))
            (goto _label)
            (else
              (bind _returnvalue_3 (Class|Inventory|GetItemsArray (Variables|/Script/LTMV.FPCharacter|Get_Inventory _asfpcharacter)))
              (bind _array_element (Utilities|Array|ForEachLoopwithBreak _returnvalue_3)
                (:LoopBody
                  (if (== _array_element (Variables|Default|GetTablilla))
                    (goto _label)))))))))
    (:CastFailed
      (bind _asvrcharacter (Utilities|Casting|CastToVRCharacter OtherActor))
      (bind _array_element_2 (Utilities|Array|ForEachLoopwithBreak (Actor|GetComponentsbyTag _asvrcharacter "/Script/Engine.StaticMeshComponent" "TablillaLaberinto"))
        (:LoopBody
          (if (== _array_element_2 (Variables|Default|GetTablilla))
            (goto _label)))))))

(event EventBeginPlay
  (Variables|Default|SetHasTablilla false)
  (bind _outactors (Actor|GetAllActorswithTag "TablillaLaberinto"))
  (bind _array_element (Utilities|Array|ForEachLoopwithBreak _outactors :!label _label)
    (:LoopBody
      (Variables|Default|SetTablilla _array_element)
      (goto _label Break))
    (:Completed
      (bind _array_element_2 (Utilities|Array|ForEachLoopwithBreak (Utilities|Struct|BreakSwitcher (Variables|/Script/LTMV.UseSwitcher|Get_SwitcherPressed (Variables|Default|GetUseSwitcher))) :!label _label_2)
        (:LoopBody
          (Variables|Default|SetDoorState_MuroFinal (Actor|GetComponentbyClass (._actor (Utilities|Struct|BreakSwitcheable _array_element_2)) "/Script/LTMV.DoorState"))
          (goto _label_2 Break))))))

(event EventUsePressed
  (Development|PrintText "PulsoAltar")
  (if (Variables|Default|GetHasTablilla)
    (if (Variables|/Script/LTMV.InventoryItem|Get_equipped (Actor|GetComponentbyClass (Variables|Default|GetTablilla) "/Script/LTMV.InventoryItem"))
      (Variables|/Script/LTMV.DoorState|Set_block (Variables|Default|GetDoorState_MuroFinal) false)
      (Transformation|DetachFromActor (Variables|Default|GetTablilla) "KeepRelative" "KeepRelative" "KeepRelative")
      (Transformation|AttachComponentToComponent (Variables|Default|GetTablilla) (Variables|Debug|GetStaticMeshComponent) "TablillaSocket" "SnapToTarget" "SnapToTarget" "KeepRelative" true))))

(fn ConstructionScript)