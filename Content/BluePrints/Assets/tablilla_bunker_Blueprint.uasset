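; Bunker tablet (tablilla) Blueprint that acts as the payoff of a four-door combination puzzle.
; Every Tick it reads the DoorState component on four referenced gates (Compuertas), looking for the pattern open, closed, open, open.
; On a match it sets the Combination flag and calls CombinationCorrect, which enables actor collision and physics simulation on its static mesh.
; Nothing resets the flag after BeginPlay, and the call repeats each frame the pattern holds.
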(event Custom|CombinationCorrect
  (if (Variables|CompuertasLaberinto|GetCombination)
    (Collision|SetActorEnableCollision true)
    (Physics|SetSimulatePhysics (Variables|Debug|GetStaticMeshComponent) true)))

(event EventTick
  (params (DeltaSeconds :type Float%20%28single-precision%29))
  (if (Math|Boolean|ANDBoolean (Utilities|Enum|Equal(Enum) (Variables|/Script/LTMV.DoorState|GetStateDoor (Actor|GetComponentbyClass (Variables|CompuertasLaberinto|GetCompuerta%201) "/Script/LTMV.DoorState")) "OPEN") (Utilities|Enum|Equal(Enum) (Variables|/Script/LTMV.DoorState|GetStateDoor (Actor|GetComponentbyClass (Variables|CompuertasLaberinto|GetCompuerta%202) "/Script/LTMV.DoorState")) "CLOSE") (Utilities|Enum|Equal(Enum) (Variables|/Script/LTMV.DoorState|GetStateDoor (Actor|GetComponentbyClass (Variables|CompuertasLaberinto|GetCompuerta%203) "/Script/LTMV.DoorState")) "OPEN") (Utilities|Enum|Equal(Enum) (Variables|/Script/LTMV.DoorState|GetStateDoor (Actor|GetComponentbyClass (Variables|CompuertasLaberinto|GetCompuerta%204) "/Script/LTMV.DoorState")) "OPEN"))
    (Variables|CompuertasLaberinto|SetCombination true)
    (CallFunction|CombinationCorrect)))

(event EventBeginPlay
  (Variables|CompuertasLaberinto|SetCombination false))

(fn ConstructionScript)