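; EndGameTrigger_Bp is a trigger actor that ends the game when a PlayerCharacter overlaps it.
; On the server, it loops over the players counted by GameModePlay and calls FadeDisplay on each FPCharacter_BP or VRCharacter_BP, covering both first-person and VR pawns.
; After a delay of about five seconds following the fade calls, it calls EndGame on GameModePlay.
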(event Collision|EventActorBeginOverlap
  (params (OtherActor :type Actor%20Object%20Reference))
  ;[1 1 1] Start Match
  (Utilities|Casting|CastToPlayerCharacter OtherActor)
  (if (Networking|IsServer)
    (bind _asgame_mode_play (Utilities|Casting|CastToGameModePlay (Game|GetGameMode)))
    (bind _returnvalue (Class|GameModeBase|GetNumPlayers _asgame_mode_play))
    (for _index (range 0 (+ _returnvalue -1))
      (bind _asfpcharacter_bp (Utilities|Casting|CastToFPCharacter_BP (Game|GetPlayerCharacter _index))
        (:then
          (Class|FPCharacter|FadeDisplay _asfpcharacter_bp))
        (:CastFailed
          (bind _asvrcharacter_bp (Utilities|Casting|CastToVRCharacter_BP (Game|GetPlayerCharacter _index)))
          (Class|VRCharacter|FadeDisplay _asvrcharacter_bp))))
    (Utilities|FlowControl|Delay 5.1)
    (Class|GameModePlay|EndGame _asgame_mode_play)))

(fn ConstructionScript)