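; Grate controller that locks or unlocks a door depending on whether the character carries the labyrinth tablet.
; BeginPlay caches the actor tagged TablillaLaberinto and the DoorState of the Switcher's first switchable actor.
; Two trigger boxes share one check: FP hands and inventory, or VR tagged mesh components.
; A match unblocks the door; otherwise an open door gets its Switcher activated and is blocked.
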(event OnComponentBeginOverlap(Box1)
  (params (OverlappedComponent :type Primitive%20Component%20Object%20Reference) (OtherActor :type Actor%20Object%20Reference) (OtherComp :type Primitive%20Component%20Object%20Reference) (OtherBodyIndex :type Integer) (bFromSweep :type Boolean) (SweepResult :type Hit%20Result%20Structure%20%28by%20ref%29))
  (bind _asfpcharacter (Utilities|Casting|CastToFPCharacter OtherActor)
    (:then
      (bind _returnvalue (Class|PlayerCharacter|GetItemLeft _asfpcharacter))
      (if (== _returnvalue (Variables|Default|GetTablilla))
        ;[1 1 1] Actua sobre la puerta en funcion de si el Character tiene o no la Tablilla
        (Variables|/Script/LTMV.DoorState|Set_block (Variables|Default|GetDoorStateReja) false :!label _label)
        (else
          (bind _returnvalue_2 (Class|PlayerCharacter|GetItemRight _asfpcharacter))
          (if (== _returnvalue_2 (Variables|Default|GetTablilla))
            (goto _label)
            (else
              (bind _returnvalue_3 (Class|Inventory|GetItemsArray (Variables|/Script/LTMV.FPCharacter|Get_Inventory _asfpcharacter)))
              (bind _array_element (Utilities|Array|ForEachLoopwithBreak _returnvalue_3)
                (:LoopBody
                  (if (== _array_element (Variables|Default|GetTablilla))
                    (goto _label)))
                (:Completed
                  (if (Utilities|Enum|Equal(Enum) (Variables|/Script/LTMV.DoorState|GetStateDoor (Variables|Default|GetDoorStateReja)) "OPEN") :!label _label_2
                    (Class|SwitcherComponent|ActivateSwitcher (Variables|Default|GetSwitcher))
                    (Variables|/Script/LTMV.DoorState|Set_block (Variables|Default|GetDoorStateReja) true)))))))))
    (:CastFailed
      (bind _asvrcharacter (Utilities|Casting|CastToVRCharacter OtherActor))
      (bind _array_element_2 (Utilities|Array|ForEachLoopwithBreak (Actor|GetComponentsbyTag _asvrcharacter "/Script/Engine.StaticMeshComponent" "TablillaLaberinto"))
        (:LoopBody
          (if (== _array_element_2 (Variables|Default|GetTablilla))
            (goto _label)))
        (:Completed
          (goto _label_2))))))

(event OnComponentBeginOverlap(Box)
  (params (OverlappedComponent :type Primitive%20Component%20Object%20Reference) (OtherActor :type Actor%20Object%20Reference) (OtherComp :type Primitive%20Component%20Object%20Reference) (OtherBodyIndex :type Integer) (bFromSweep :type Boolean) (SweepResult :type Hit%20Result%20Structure%20%28by%20ref%29))
  (bind _asfpcharacter (Utilities|Casting|CastToFPCharacter OtherActor)
    (:then
      (bind _returnvalue (Class|PlayerCharacter|GetItemLeft _asfpcharacter))
      (if (== _returnvalue (Variables|Default|GetTablilla))
        ;[1 1 1] Actua sobre la puerta en funcion de si el Character tiene o no la Tablilla
        (Variables|/Script/LTMV.DoorState|Set_block (Variables|Default|GetDoorStateReja) false :!label _label)
        (else
          (bind _returnvalue_2 (Class|PlayerCharacter|GetItemRight _asfpcharacter))
          (if (== _returnvalue_2 (Variables|Default|GetTablilla))
            (goto _label)
            (else
              (bind _returnvalue_3 (Class|Inventory|GetItemsArray (Variables|/Script/LTMV.FPCharacter|Get_Inventory _asfpcharacter)))
              (bind _array_element (Utilities|Array|ForEachLoopwithBreak _returnvalue_3)
                (:LoopBody
                  (if (== _array_element (Variables|Default|GetTablilla))
                    (goto _label)))
                (:Completed
                  (if (Utilities|Enum|Equal(Enum) (Variables|/Script/LTMV.DoorState|GetStateDoor (Variables|Default|GetDoorStateReja)) "OPEN") :!label _label_2
                    (Class|SwitcherComponent|ActivateSwitcher (Variables|Default|GetSwitcher))
                    (Variables|/Script/LTMV.DoorState|Set_block (Variables|Default|GetDoorStateReja) true)))))))))
    (:CastFailed
      (bind _asvrcharacter (Utilities|Casting|CastToVRCharacter OtherActor))
      (bind _array_element_2 (Utilities|Array|ForEachLoopwithBreak (Actor|GetComponentsbyTag _asvrcharacter "/Script/Engine.StaticMeshComponent" "TablillaLaberinto"))
        (:LoopBody
          (if (== _array_element_2 (Variables|Default|GetTablilla))
            (goto _label)))
        (:Completed
          (goto _label_2))))))

(event EventBeginPlay
  (bind _outactors (Actor|GetAllActorswithTag "TablillaLaberinto"))
  (bind _array_element (Utilities|Array|ForEachLoopwithBreak _outactors :!label _label)
    (:LoopBody
      (Variables|Default|SetTablilla _array_element)
      (goto _label Break))
    (:Completed
      (bind _array_element_2 (Utilities|Array|ForEachLoopwithBreak (Utilities|Struct|BreakSwitcher (Variables|/Script/LTMV.SwitcherComponent|Get_Switcher (Variables|Default|GetSwitcher))) :!label _label_2)
        (:LoopBody
          (Variables|Default|SetDoorStateReja (Actor|GetComponentbyClass (._actor (Utilities|Struct|BreakSwitcheable _array_element_2)) "/Script/LTMV.DoorState"))
          (goto _label_2 Break))))))

(fn ConstructionScript)