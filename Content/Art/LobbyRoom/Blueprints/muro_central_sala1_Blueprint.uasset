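; Central wall Blueprint for room 1 of the lobby that links two wall traps to a door.
; Tick polls both trap states and, while both are Pressed, sends a switch-state message to the door and plays a sound at the world origin.
; No latch guards the check, so the message and sound repeat every frame the condition holds.
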(event EventTick
  (params (DeltaSeconds :type Float%20%28single-precision%29))
  (if (and (Utilities|Enum|Equal(Enum) (Variables|/Script/LTMV.WallTrapState|Get_State (Variables|Default|GetWallTrapState1)) "Pressed") (Utilities|Enum|Equal(Enum) (Variables|/Script/LTMV.WallTrapState|Get_State (Variables|Default|GetWallTrapState)) "Pressed"))
    (Class|ItfSwitcheable|SwitchState(Message) (Variables|Default|GetDoorState))
    (Audio|PlaySoundatLocation 0 "0, 0, 0")))

(fn ConstructionScript)