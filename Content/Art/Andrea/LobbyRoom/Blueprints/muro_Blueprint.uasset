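; Lobby room wall Blueprint that activates a switcher once two wall traps are both pressed.
; Tick polls the State of both referenced traps and calls ActivateSwitcher when both read Pressed.
; An Executed flag makes the trigger fire only once.
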(event EventTick
  (params (DeltaSeconds :type Float%20%28single-precision%29))
  (if (not (Variables|Default|GetExecuted))
    (if (and (Utilities|Enum|Equal(Enum) (Variables|/Script/LTMV.WallTrapState|Get_State (Variables|Default|GetWallTrapState1)) "Pressed") (Utilities|Enum|Equal(Enum) (Variables|/Script/LTMV.WallTrapState|Get_State (Variables|Default|GetWallTrapState)) "Pressed"))
      (Class|SwitcherComponent|ActivateSwitcher (Variables|Default|GetSwitcher))
      (Variables|Default|SetExecuted true))))

(fn ConstructionScript)